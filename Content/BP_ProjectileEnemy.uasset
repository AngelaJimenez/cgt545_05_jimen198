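; BP_ProjectileEnemy is an enemy projectile that damages the player character on hit and destroys itself five seconds after spawning.
; BeginPlay plays an explosion sound at the world origin rather than at the projectile, then starts the lifetime delay.
; Mesh hits print the other actor's name and call DamageCharacter if it is the first BP_FirstPersonCharacter found through GetAllActorsOfClass, without destroying the projectile.
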(event `self.ReceiveBeginPlay`
  (`GameplayStatics.PlaySoundAtLocation` "/Game/StarterContent/Audio/Explosion01.Explosion01" (0.0 0.0 0.0) (struct) 1.0 1.0 0.0 null null null null)
  ;[1 1 1] Failed
  (`KismetSystemLibrary.Delay` 5.0)
  (`self.K2_DestroyActor`))

(event `self.StaticMeshComponent.OnComponentBeginOverlap`
  (params (OverlappedComponent :type "PrimitiveComponent Object Reference") (OtherActor :type "Actor Object Reference") (OtherComp :type "PrimitiveComponent Object Reference") (OtherBodyIndex :type Integer) (bFromSweep :type Boolean) (SweepResult :type "HitResult Structure (by ref)")))

(event `self.StaticMeshComponent.OnComponentHit`
  (params (HitComponent :type "PrimitiveComponent Object Reference") (OtherActor :type "Actor Object Reference") (OtherComp :type "PrimitiveComponent Object Reference") (NormalImpulse :type "Vector Structure") (Hit :type "HitResult Structure (by ref)"))
  ;[1 1 1] Failed
  (`KismetSystemLibrary.PrintText` (`KismetTextLibrary.Conv_StringToText` (`KismetSystemLibrary.GetDisplayName` OtherActor)))
  (bind _outactors (`GameplayStatics.GetAllActorsOfClass` "/Game/FirstPerson/Blueprints/BP_FirstPersonCharacter.BP_FirstPersonCharacter_C"))
  (bind _output (`|GetArrayItem` _outactors))
  (if (== OtherActor _output)
    (`/Game/FirstPerson/Blueprints/BP_FirstPersonCharacter.DamageCharacter` _output)))

(fn `UserConstructionScript`)