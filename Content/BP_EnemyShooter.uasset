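; BP_EnemyShooter is an enemy that fires a projectile at the first-person character roughly every three seconds.
; Tick feeds a Delay that paces the shots, then looks up the first BP_FirstPersonCharacter in the level.
; It spawns BP_ProjectileEnemy at its own location, rotated toward the player, and applies an impulse to the projectile's mesh.
; The impulse uses the unnormalized offset to the player, so its strength grows with distance.
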(event `self.ReceiveTick`
  (params (DeltaSeconds :type "Float (single-precision)"))
  (bind _returnvalue (`self.K2_GetActorLocation`))
  (`KismetSystemLibrary.Delay` 3.0)
  (bind _outactors (`GameplayStatics.GetAllActorsOfClass` "/Game/FirstPerson/Blueprints/BP_FirstPersonCharacter.BP_FirstPersonCharacter_C"))
  (bind _returnvalue_2 (`self.K2_GetActorLocation` (`|GetArrayItem` _outactors)))
  (bind _returnvalue_3 (`|SpawnActorFromClass` "/Game/BP_ProjectileEnemy.BP_ProjectileEnemy_C" (`KismetMathLibrary.MakeTransform` (`self.K2_GetActorLocation`) (`KismetMathLibrary.FindLookAtRotation` _returnvalue _returnvalue_2)) "Undefined" "MultiplyWithRoot" null null))
  (`PrimitiveComponent.AddImpulse` (`StaticMeshActor.StaticMeshComponent` _returnvalue_3) (* (- _returnvalue_2 _returnvalue) 3000.0) "None" false))

(fn `UserConstructionScript`)